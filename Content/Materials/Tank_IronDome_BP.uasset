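; Player-controlled tank pawn Blueprint, an Iron Dome variant that drives on two tracks and aims and fires through a dedicated aiming component.
; BeginPlay hands the barrel and turret to TankAimingComponentIronDome and both tracks to TankMovement.
; Input axes rotate the azimuth gimbal and spring arm and send movement intents, while Fire calls both Launch and Fire.
; The construction script assigns barrel and track meshes plus a track physical material override.
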(event `self.ReceiveBeginPlay`
  (`TankAimingComponent.Initialize` (`self.TankAimingComponentIronDome`) (`self.Barrel`) (`self.Turret`))
  (`TankMovementComponent.Initialize` (`self.TankMovement`) (`self.LeftTrack`) (`self.RightTrack`)))

(event `InputAxis|AimAzimuth`
  (params (AxisValue :type "Float (single-precision)"))
  ;[1 1 1] Aim Input Binding
  (`SceneComponent.K2_AddLocalRotation` (`self.AzimuthGimbal`) (`KismetMathLibrary.MakeRotator` 0.0 0.0 AxisValue) false false))

(event `InputAxis|MoveForward`
  (params (AxisValue :type "Float (single-precision)"))
  ;[1 1 1] Simple Movement Input
  (`TankMovementComponent.IntentMoveForward` (`self.TankMovement`) AxisValue))

(event `InputAxis|AimElevation`
  (params (AxisValue :type "Float (single-precision)"))
  ;[1 1 1] Aim Input Binding
  (`SceneComponent.K2_AddLocalRotation` (`self.SpringArm`) (`KismetMathLibrary.MakeRotator` 0.0 AxisValue) false false))

(event `InputAxis|Turn Right`
  (params (AxisValue :type "Float (single-precision)"))
  ;[1 1 1] Simple Movement Input
  (`TankMovementComponent.IntentTurnRight` (`self.TankMovement`) AxisValue))

(event `InputAction|Fire`
  (params (Key :type "Key Structure"))
  ;[1 1 1] Aim Input Binding
  (:`Pressed`
    (`TankAimingComponentIronDome.Launch` (`self.TankAimingComponentIronDome`))
    (`TankAimingComponent.Fire` (`self.TankAimingComponentIronDome`))))

(fn `UserConstructionScript`
  (`StaticMeshComponent.SetStaticMesh` (`self.Barrel`) "/Game/Materials/tank_fbx_Barrel_cannon.tank_fbx_Barrel_cannon")
  (`StaticMeshComponent.SetStaticMesh` (`self.LeftTrack`) "/Game/Materials/tank_fbx_Track_track_001.tank_fbx_Track_track_001")
  (`StaticMeshComponent.SetStaticMesh` (`self.RightTrack`) "/Game/Materials/tank_fbx_Track_track_001.tank_fbx_Track_track_001")
  (`PrimitiveComponent.SetPhysMaterialOverride` (`self.RightTrack`) "/Game/Materials/Track.Track")
  (`PrimitiveComponent.SetPhysMaterialOverride` (`self.LeftTrack`) "/Game/Materials/Track.Track"))