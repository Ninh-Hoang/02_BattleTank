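; Enemy projectile Blueprint that can be shot down by other projectiles.
; On actor overlap it checks whether the other actor's class is exactly Projectile_BP or Rocket_Tank_BP, combining the two tests with an integer bitwise OR.
; On a match it prints that actor's name and destroys only itself.
; The graphs hold no movement or damage logic.
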(event `self.ReceiveActorBeginOverlap`
  (params (OtherActor :type "Actor Object Reference"))
  (bind _returnvalue (`GameplayStatics.GetObjectClass` OtherActor))
  (if (`KismetMathLibrary.Conv_IntToBool` (`KismetMathLibrary.Or_IntInt` (`KismetMathLibrary.Conv_BoolToInt` (== _returnvalue "/Game/Materials/Projectile_BP.Projectile_BP_C")) (`KismetMathLibrary.Conv_BoolToInt` (== _returnvalue "/Game/Materials/Rocket_Tank_BP.Rocket_Tank_BP_C"))))
    (`KismetSystemLibrary.PrintString` (`KismetSystemLibrary.GetObjectName` OtherActor))
    (`self.K2_DestroyActor`)))

(fn `UserConstructionScript`)