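; Player-drivable tank with an automatic CIWS-style gun that aims and fires at the projectile reported by its TankAiming component.
; Each Tick it predicts a shot path toward that projectile, derives a flight time from the hit segment, and forward-simulates the projectile to get an intercept point, drawing debug spheres and printing it.
; Input drives TankMovement, camera gimbal and manual fire; construction sets barrel and track meshes.
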(event `self.ReceiveTick`
  (params (DeltaSeconds :type "Float (single-precision)"))
  (bind _tankaiming1 (`self.TankAiming1`))
  (bind _returnvalue (`SceneComponent.GetSocketLocation` (`self.Barrel`) "Projectile"))
  (bind _returnvalue_2 (`TankAimingComponent.GetProjectile` (`self.TankAiming1`)))
  (if (`KismetSystemLibrary.IsValid` _returnvalue_2)
    (bind _returnvalue_3 (`self.K2_GetActorLocation` _returnvalue_2))
    (bind _tossvelocity (`GameplayStatics.BlueprintSuggestProjectileVelocity` _returnvalue _returnvalue_3 40000.0 0.0 "DoNotTrace"))
    (bind _predictresult (`GameplayStatics.Blueprint_PredictProjectilePath_Advanced` (make `PredictProjectilePathParams` _returnvalue _tossvelocity true 0.0 1.0 true "ECC_WorldDynamic" (`|MakeArray` "ObjectTypeQuery7" :!type "EObjectTypeQuery Enum") (`|MakeArray` null :!type "Actor Object Reference"))))
    (bind (_pathdata _lasttracedestination _hitresult) (break `PredictProjectilePathResult` _predictresult))
    (for (_array_element _array_index) _pathdata
      (bind (_bblockinghit _binitialoverlap _time _distance _location _impactpoint _normal _impactnormal _physmat _hitactor _hitcomponent _hitbonename _hititem _faceindex _tracestart) (`GameplayStatics.BreakHitResult` _hitresult))
      (if (== (`.Location` (break `PredictProjectilePathPointData` _array_element)) _tracestart)
        (bind _predictresult_2 (`GameplayStatics.Blueprint_PredictProjectilePath_Advanced` (make `PredictProjectilePathParams` _returnvalue_3 (`self.GetVelocity` _returnvalue_2) true 0.0 (/ (+ (`KismetMathLibrary.Conv_IntToDouble` _array_index) _time) 20.0) true "ECC_GameTraceChannel1" (`|MakeArray` "ObjectTypeQuery4" :!type "EObjectTypeQuery Enum") (`|MakeArray` null :!type "Actor Object Reference"))))
        (bind (_pathdata_2 _lasttracedestination_2 _hitresult_2) (break `PredictProjectilePathResult` _predictresult_2))
        (`KismetSystemLibrary.DrawDebugSphere` (`.Location` (`GameplayStatics.BreakHitResult` _hitresult_2)) 200.0 12 (struct :`G` 0.895292 :`B` 1.0 :`A` 1.0))
        (`KismetSystemLibrary.DrawDebugSphere` (0.0 0.0 0.0) 200.0 12 (struct :`G` 0.895292 :`B` 1.0 :`A` 1.0))
        (bind (_location_2 _velocity _time_2) (break `PredictProjectilePathPointData` _lasttracedestination_2))
        (`KismetSystemLibrary.PrintString` (`KismetStringLibrary.Conv_VectorToString` _location_2))
        (`TankAimingComponent.AimAt` _tankaiming1 _location_2)
        (`TankAimingComponent.Fire` _tankaiming1)))))

(event `self.ReceiveBeginPlay`
  ;[1 1 1] BeginPlay
  (`TankAimingComponent.Initialize` (`self.TankAiming1`) (`self.Barrel`) (`self.Turret`))
  (`TankMovementComponent.Initialize` (`self.TankMovement`) (`self.LeftTrack`) (`self.RightTrack`)))

(event `InputAxis|AimAzimuth`
  (params (AxisValue :type "Float (single-precision)"))
  ;[1 1 1] Aim Input Binding
  (`SceneComponent.K2_AddLocalRotation` (`self.AzimuthGimbal`) (`KismetMathLibrary.MakeRotator` 0.0 0.0 AxisValue) false false))

(event `InputAxis|MoveForward`
  (params (AxisValue :type "Float (single-precision)"))
  ;[1 1 1] Simple Movement Input
  (`TankMovementComponent.IntentMoveForward` (`self.TankMovement`) AxisValue))

(event `InputAxis|AimElevation`
  (params (AxisValue :type "Float (single-precision)"))
  ;[1 1 1] Aim Input Binding
  (`SceneComponent.K2_AddLocalRotation` (`self.SpringArm`) (`KismetMathLibrary.MakeRotator` 0.0 AxisValue) false false))

(event `InputAxis|Turn Right`
  (params (AxisValue :type "Float (single-precision)"))
  ;[1 1 1] Simple Movement Input
  (`TankMovementComponent.IntentTurnRight` (`self.TankMovement`) AxisValue))

(event `InputAction|Fire`
  (params (Key :type "Key Structure"))
  ;[1 1 1] Aim Input Binding
  (:`Pressed`
    (`TankAimingComponent.Fire` (`self.TankAiming1`))))

(fn `UserConstructionScript`
  (`StaticMeshComponent.SetStaticMesh` (`self.Barrel`) "/Game/Materials/tank_fbx_Barrel_cannon.tank_fbx_Barrel_cannon")
  (`StaticMeshComponent.SetStaticMesh` (`self.LeftTrack`) "/Game/Materials/tank_fbx_Track_track_001.tank_fbx_Track_track_001")
  (`StaticMeshComponent.SetStaticMesh` (`self.RightTrack`) "/Game/Materials/tank_fbx_Track_track_001.tank_fbx_Track_track_001")
  (`PrimitiveComponent.SetPhysMaterialOverride` (`self.RightTrack`) "/Game/Materials/Track.Track")
  (`PrimitiveComponent.SetPhysMaterialOverride` (`self.LeftTrack`) "/Game/Materials/Track.Track"))